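; MyGameInstance stores the player's inventory of coins and Equipment, Consumable and Material item arrays.
; Each item carries a slot index, so arrays hold only occupied slots, with inserts positioned by that index.
; Adding increments an existing stack or fills the first free slot, up to InventorySize.
; Swapping exchanges two items or moves one to an empty slot via set, remove and insert helpers, which call CallRefreshItem.
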(fn GetInventoryItemArrayIndex
  (params (ByID? :type Boolean) (ID :type Integer) (ByInventoryIndex? :type Boolean) (InventoryIndex :type Integer) (PropType :type E_PropType%20Enum :default "NewEnumerator0"))
  (if ByID?
    (bind _items (CallFunction|GetInventorybyType PropType))
    (for (_array_element _array_index) _items
      (if (== (.ID (Utilities|Struct|BreakS_InventoryItem _array_element)) ID)
        (return true _array_index)))
    (return false 0)
    (else
      (if ByInventoryIndex?
        (bind _items_2 (CallFunction|GetInventorybyType PropType))
        (for (_array_element_2 _array_index_2) _items_2
          (if (== (.Index (Utilities|Struct|BreakS_InventoryItem _array_element_2)) InventoryIndex)
            (return true _array_index_2))))
      (return false 0))))

(fn SetInventoryItem
  (params (Type :type E_PropType%20Enum :default "NewEnumerator0") (ArrayIndex :type Integer) (New%20Item :type S%20Inventory%20Item%20Structure))
  (bind _inventory (Variables|Default|GetInventory))
  (bind (_coins _equipment _consumable _material) (Utilities|Struct|BreakS_Inventory _inventory))
  (bind _returnvalue (Utilities|Select :Index Type :NewEnumerator0 _equipment :NewEnumerator2 _consumable :NewEnumerator1 _material))
  (if (Utilities|Array|IsValidIndex _returnvalue ArrayIndex)
    (Utilities|Array|SetArrayElem _returnvalue ArrayIndex New%20Item)
    (Default|CallRefreshItem "NewEnumerator0" Type New%20Item)
    (return true)
    (else
      (return false))))

(fn RemoveInventoryItem
  (params (Type :type E_PropType%20Enum :default "NewEnumerator0") (ArrayIndex :type Integer))
  (bind _inventory (Variables|Default|GetInventory))
  (bind (_coins _equipment _consumable _material) (Utilities|Struct|BreakS_Inventory _inventory))
  (bind _returnvalue (Utilities|Select :Index Type :NewEnumerator0 _equipment :NewEnumerator2 _consumable :NewEnumerator1 _material))
  (if (Utilities|Array|IsValidIndex _returnvalue ArrayIndex)
    (Default|CallRefreshItem "NewEnumerator0" Type (Utilities|Struct|MakeS_InventoryItem (.Index (Utilities|Struct|BreakS_InventoryItem (Utilities|Array|Get(acopy) _returnvalue ArrayIndex)))))
    (Utilities|Array|RemoveIndex _returnvalue ArrayIndex)
    (return true)
    (else
      (return false))))

(fn InsertNewInventoryItem
  (params (Type :type E_PropType%20Enum :default "NewEnumerator0") (ArrayIndex :type Integer) (New%20Item :type S%20Inventory%20Item%20Structure))
  (bind _inventory (Variables|Default|GetInventory))
  (bind _inventorysize (Variables|Default|GetInventorySize))
  (bind (_coins _equipment _consumable _material) (Utilities|Struct|BreakS_Inventory _inventory))
  (bind _returnvalue (Utilities|Select :Index Type :NewEnumerator0 _equipment :NewEnumerator2 _consumable :NewEnumerator1 _material))
  (if (< (Utilities|Array|Length _returnvalue) _inventorysize)
    (if (Math|Integer|InRange(Integer) ArrayIndex 0 _inventorysize true false)
      (Utilities|Array|Insert _returnvalue New%20Item ArrayIndex)
      (Default|CallRefreshItem "NewEnumerator0" Type New%20Item)
      (return true "")
      (else
        (return false "超出最大位置")))
    (else
      (return false "背包满了"))))

(fn GetInventoryInsertArrayIndex
  (params (KnowIndex? :type Boolean) (Type :type E_PropType%20Enum :default "NewEnumerator0") (InsertIndex :type Integer))
  (if KnowIndex?
    (LocalVariables|SetLocalInventoryIndex InsertIndex)
    (else
      (LocalVariables|SetLocalInventoryIndex 0)))
  (bind _items (CallFunction|GetInventorybyType Type))
  (bind (_array_element _array_index) (Utilities|Array|ForEachLoopwithBreak _items :!label _label)
    (:LoopBody
      (if (< (LocalVariables|GetLocalInventoryIndex) (.Index (Utilities|Struct|BreakS_InventoryItem _array_element)))
        (LocalVariables|SetLocalInsertIndex _array_index)
        (LocalVariables|SetLocal%20Find? true)
        (goto _label Break)
        (elif (not KnowIndex?)
          (LocalVariables|SetLocalInventoryIndex (+ (.Index (Utilities|Struct|BreakS_InventoryItem _array_element)) 1)))))
    (:Completed
      (if (LocalVariables|GetLocal%20Find?)
        (return (LocalVariables|GetLocalInventoryIndex) (LocalVariables|GetLocalInsertIndex))
        (else
          (return (LocalVariables|GetLocalInventoryIndex) (Utilities|Array|Length _items)))))))

(fn AddInventoryItem
  (params (Props :type S%20Props%20Structure))
  (bind (_id _name _proptype) (Utilities|Struct|BreakS_Props Props))
  (bind _inventory (Variables|Default|GetInventory))
  (bind (_coins _equipment _consumable _material) (Utilities|Struct|BreakS_Inventory _inventory))
  (bind _array_element (Utilities|Array|ForEachLoopwithBreak (Utilities|Select :Index _proptype :NewEnumerator0 _equipment :NewEnumerator2 _consumable :NewEnumerator1 _material) :!label _label)
    (:LoopBody
      (if (== (.ID (Utilities|Struct|BreakS_InventoryItem _array_element)) _id)
        (LocalVariables|SetLoc%20Find true)
        (Math|Integer|IncrementInt (.Quantities (Utilities|Struct|BreakS_InventoryItem _array_element))
          (:%20%20
            (goto _label Break)))))
    (:Completed
      (if (LocalVariables|GetLoc%20Find)
        (Default|CallRefreshItem "NewEnumerator0" _proptype _array_element)
        (return true)
        (else
          (bind (_insertinventoryindex _insertarrayindex) (Inventory|GetInventoryInsertArrayIndex false _proptype))
          (bind _success_ (Inventory|InsertNewInventoryItem _proptype _insertarrayindex (Utilities|Struct|MakeS_InventoryItem _insertinventoryindex _id 1)))
          (return _success_))))))

(fn GetCoins
  (return (.Coins (Utilities|Struct|BreakS_Inventory (Variables|Default|GetInventory)))))

(fn GetInventorybyType
  (params (Type :type E_PropType%20Enum :default "NewEnumerator0"))
  (bind _inventory (Variables|Default|GetInventory))
  (bind (_coins _equipment _consumable _material) (Utilities|Struct|BreakS_Inventory _inventory))
  (return (Utilities|Select :Index Type :NewEnumerator0 _equipment :NewEnumerator2 _consumable :NewEnumerator1 _material)))

(fn GetInventorysize
  (return (Variables|Default|GetInventorySize)))

(fn SwapPropI2I
  (params (Item_1_Valid :type Boolean) (Item_2_Valid :type Boolean) (InventoryItem_1 :type S%20Inventory%20Item%20Structure) (InventoryItem_2 :type S%20Inventory%20Item%20Structure) (PropType :type E_PropType%20Enum :default "NewEnumerator0"))
  (bind (_index _id _quantities) (Utilities|Struct|BreakS_InventoryItem InventoryItem_2))
  (bind (_index_2 _id_2 _quantities_2) (Utilities|Struct|BreakS_InventoryItem InventoryItem_2))
  (bind (_index_3 _id_3 _quantities_3) (Utilities|Struct|BreakS_InventoryItem InventoryItem_1))
  (bind (_index_4 _id_4 _quantities_4) (Utilities|Struct|BreakS_InventoryItem InventoryItem_1))
  (if Item_1_Valid
    (bind (_found_ _array_index) (Inventory|GetInventoryItemArrayIndex false 0 true (.Index (Utilities|Struct|BreakS_InventoryItem InventoryItem_1)) PropType))
    (if _found_
      (LocalVariables|SetLocalItem1ArrayIndex _array_index)
      (if Item_2_Valid
        (bind (_found__2 _array_index_2) (Inventory|GetInventoryItemArrayIndex false 0 true (.Index (Utilities|Struct|BreakS_InventoryItem InventoryItem_2)) PropType))
        (if _found__2
          (bind _output_get (LocalVariables|SetLocalItem2ArrayIndex _array_index_2))
          (bind _success_ (Inventory|SetInventoryItem PropType _output_get (Utilities|Struct|MakeS_InventoryItem (.Index (Utilities|Struct|BreakS_InventoryItem InventoryItem_2)) _id_3 _quantities_3))) ; Set Item2
          (if _success_
            (bind _success__2 (Inventory|SetInventoryItem PropType (LocalVariables|GetLocalItem1ArrayIndex) (Utilities|Struct|MakeS_InventoryItem (.Index (Utilities|Struct|BreakS_InventoryItem InventoryItem_1)) _id_2 _quantities_2))) ; Set Item1
            (return _success__2 "")
            (else
              (return false "Set Error")))
          (else
            (return false "Not Found Item2")))
        (else
          (bind _success__3 (Inventory|RemoveInventoryItem PropType (LocalVariables|GetLocalItem1ArrayIndex)))
          (if _success__3
            (bind (_insertinventoryindex _insertarrayindex) (Inventory|GetInventoryInsertArrayIndex true PropType (.Index (Utilities|Struct|BreakS_InventoryItem InventoryItem_2))))
            (bind (_success__4 _reason) (Inventory|InsertNewInventoryItem PropType _insertarrayindex (Utilities|Struct|MakeS_InventoryItem _insertinventoryindex _id_4 _quantities_4)))
            (return _success__4 _reason)
            (else
              (return false "Fail to Remove Item1")))))
      (else
        (return false "Not Found Item1")))
    (elif Item_2_Valid
      (bind (_found__3 _array_index_3) (Inventory|GetInventoryItemArrayIndex false 0 true (.Index (Utilities|Struct|BreakS_InventoryItem InventoryItem_2)) PropType))
      (if _found__3
        (bind _output_get_2 (LocalVariables|SetLocalItem2ArrayIndex _array_index_3))
        (Inventory|RemoveInventoryItem PropType _output_get_2)
        (if true
          (bind (_insertinventoryindex_2 _insertarrayindex_2) (Inventory|GetInventoryInsertArrayIndex true PropType (.Index (Utilities|Struct|BreakS_InventoryItem InventoryItem_1))))
          (bind (_success__5 _reason_2) (Inventory|InsertNewInventoryItem PropType _insertinventoryindex_2 (Utilities|Struct|MakeS_InventoryItem _insertarrayindex_2 _id _quantities)))
          (return _success__5 _reason_2)
          (else
            (return false "Remove Error")))
        (else
          (return false "Item2 Not Found")))
      (else
        (return false "Item1,2不存在")))))