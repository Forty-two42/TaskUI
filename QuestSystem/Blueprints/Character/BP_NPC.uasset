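; BP_NPC is a talkable quest-giver character that can patrol a looping list of points via AI MoveTo.
; Player proximity toggles its named interaction widget, and a question mark shows when a quest class is assigned.
; Interacting adds and starts that quest if the player's quest manager lacks it, otherwise the NPC talks.
; Talking displays a timed message, blocks re-talking meanwhile, and reports the NPC's class and ID to the quest manager.
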(event Custom|MoveToPatrolPoint
  ;[1 1 1] MovetoPatrolPoint
  (AI|AIMoveTo self (Transformation|GetActorLocation (Utilities|Array|Get(acopy) (Variables|Default|GetPatrolPoints) (Variables|Default|GetCurrentPatrolIndex))) 0 42.0 true
    (:OnSuccess
      (Variables|Default|SetCurrentPatrolIndex (select (< (Variables|Default|GetCurrentPatrolIndex) (Utilities|Array|LastIndex (Variables|Default|GetPatrolPoints))) (+ (Variables|Default|GetCurrentPatrolIndex) 1) 0))
      (CallFunction|MovetoPatrolPoint))))

(event Custom|OnTalkTo
  (params (Player :type Third%20Person%20Character%20Object%20Reference))
  ;[1 1 1] Talk
  (CallFunction|ShowMessage (Variables|Default|GetDefaultMessage) (Variables|Default|GetDefaultDuration) Player))

(event Custom|ShowMessage
  (params (Message :type Text) (Duration :type Float%20%28single-precision%29) (Player :type Third%20Person%20Character%20Object%20Reference))
  ;[1 1 1] ShowMessage
  (if (Variables|Default|GetCanBeTalked?)
    (Variables|Default|SetCanBeTalked? false)
    (Rendering|SetVisibility (Variables|Default|GetInteractionWidget) false false)
    (Rendering|Components|TextRender|SetText (Variables|/Game/QuestSystem/Blueprints/Widgets/MessageWidget.MessageWidget_C|GetMessage_Text (Variables|Default|GetMessageWidget)) Message)
    (Rendering|SetVisibility (Variables|Default|GetMessageComponent) true false)
    (Default|OnTalktoNPC (Variables|/Game/QuestSystem/Blueprints/Character/ThirdPersonCharacter.ThirdPersonCharacter_C|GetQuestManagerRef Player) (Utilities|GetClass self) (Variables|Default|GetNpcId))
    (Utilities|FlowControl|Delay Duration)
    (Rendering|SetVisibility (Variables|Default|GetMessageComponent) false false)
    (Rendering|SetVisibility (Variables|Default|GetInteractionWidget) (Variables|Default|GetInPlayerRaidus?) false)
    (Variables|Default|SetCanBeTalked? true)))

(event EventOnInteractwith
  (params (Character :type Third%20Person%20Character%20Object%20Reference))
  (bind _questmanagerref (Variables|/Game/QuestSystem/Blueprints/Character/ThirdPersonCharacter.ThirdPersonCharacter_C|GetQuestManagerRef Character))
  (bind _hasquest (Variables|Default|GetHasQuest))
  ;[1 1 1] Event Interact
  (if (Utilities|IsValidClass _hasquest)
    (if (Utilities|Array|ContainsItem (Variables|/Game/QuestSystem/Blueprints/Actors/BP_QuestManager.BP_QuestManager_C|GetAllQuestClasses _questmanagerref) _hasquest)
      (CallFunction|OnTalkto Character)
      (else
        (Default|AddNewQuest _questmanagerref (Variables|Default|GetHasQuest) true)
        (Rendering|SetVisibility (Variables|Default|GetQuestionMark) false false)))
    (else
      (CallFunction|OnTalkto Character))))

(event EventBeginPlay
  ;[1 1 1] Event BeginPlay
  (Actor|SetOwner (Game|GetPlayerCharacter 0))
  (Rendering|SetVisibility (Variables|Default|GetQuestionMark) (Utilities|IsValidClass (Variables|Default|GetHasQuest)) false)
  (Variables|Default|SetMessageWidget (.AsMessage%20Widget (Utilities|Casting|CastToMessageWidget (UserInterface|GetUserWidgetObject (Variables|Default|GetMessageComponent)))))
  (bind _asinteraction_widget (Utilities|Casting|CastToInteractionWidget (UserInterface|GetUserWidgetObject (Variables|Default|GetInteractionWidget)))
    (:then
      (Rendering|Components|TextRender|SetText (Variables|/Game/QuestSystem/Blueprints/Widgets/InteractionWidget.InteractionWidget_C|GetTextBlock_Name _asinteraction_widget) (Variables|Default|GetName)))
    (:CastFailed
      _))
  (if (and (Variables|Default|GetDoesPatrol?) (> (Utilities|Array|Length (Variables|Default|GetPatrolPoints)) 0))
    (CallFunction|MovetoPatrolPoint)))

(event EventOnEnterPlayerRadius
  (params (Character :type Third%20Person%20Character%20Object%20Reference))
  ;[1 1 1] Event Enter/Leave
  (Variables|Default|SetInPlayerRaidus? true)
  (if (Variables|Default|GetCanBeTalked?)
    (Rendering|SetVisibility (Variables|Default|GetInteractionWidget) true false)))

(event EventOnLeavePlayerRadius
  (params (Character :type Third%20Person%20Character%20Object%20Reference))
  ;[1 1 1] Event Enter/Leave
  (Variables|Default|SetInPlayerRaidus? false)
  (Rendering|SetVisibility (Variables|Default|GetInteractionWidget) false false))

(fn ConstructionScript)