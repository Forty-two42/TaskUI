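; Base enemy character for the quest system that runs a behavior tree, fights the player and can be killed for EXP.
; Sight or damage from the player flags it in the blackboard and raises walk speed.
; Attacks play a montage, with a notify line trace applying damage, then report back to the BT task.
; Death credits EXP and quest progress to the killer, triggers respawn and destroys the actor, while a widget shows name, level and health.
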(event OnSeePawn(PawnSensing)
  (params (Pawn :type Pawn%20Object%20Reference))
  ;[1 1 1] SeePlayer
  (CallFunction|OnNoticeActor Pawn))

(event Custom|EventAttack
  (params (Task_Attack :type Task%20Attack%20Object%20Reference))
  (bind _animmontage (Variables|ChildrenDefault|GetAnimMontage))
  ;[1 1 1] Attack
  (Transformation|SetActorRelativeRotation (Math|Rotator|FindLookatRotation (Transformation|GetActorLocation) (Transformation|GetActorLocation (Game|GetPlayerCharacter 0))))
  (Animation|PlayAnimMontage _animmontage 1.0 "None")
  (Utilities|FlowControl|Delay (Variables|/Script/Engine.AnimSequenceBase|GetSequenceLength _animmontage))
  (Default|EventAttackLaunched Task_Attack))

(event Custom|AttackNotify
  (bind _returnvalue (Transformation|GetActorLocation))
  ;[1 1 1] Attack
  (bind _outhit (Collision|LineTraceForObjects _returnvalue (+ _returnvalue (* (Transformation|GetActorForwardVector) (Variables|ChildrenDefault|GetActorDistance))) (Utilities|Array|MakeArray "ObjectTypeQuery3") true 0 "ForDuration"))
  (Game|Damage|ApplyDamage (.HitActor (Collision|BreakHitResult _outhit)) 2e+01 0 self))

(event Custom|On%20Death
  (bind _returnvalue (Animation|GetCurrentMontage :!class /Script/Engine.Character))
  ;[1 1 1] Death
  (Utilities|IsValid _returnvalue
    (:Is%20Valid
      (Animation|StopAnimMontage _returnvalue))
    (:Is%20Not%20Valid
      _))
  (Variables|Gameplay|SetIsDead? true)
  (AI|Components|Blackboard|SetValueasBool (AI|GetBlackboard 0) (Utilities|Name|MakeLiteralName "IsDead?") true)
  (Collision|SetCollisionEnabled (Variables|Collision|GetCapsuleComponent) "NoCollision")
  (Components|DestroyComponent (Variables|Default|GetWidget))
  (bind _asthird_person_character (Utilities|Casting|CastToThirdPersonCharacter (Variables|Gameplay|GetKilledBy))
    (:then
      (Default|AddEXPPoints _asthird_person_character (Variables|ChildrenDefault|GetExpForKill))
      (Default|OnEnemyKilled (Variables|/Game/QuestSystem/Blueprints/Character/ThirdPersonCharacter.ThirdPersonCharacter_C|GetQuestManagerRef _asthird_person_character) (Utilities|GetClass self)))
    (:CastFailed
      _))
  (Utilities|FlowControl|Delay 2.0)
  (Default|RespawnEnemy (Variables|Gameplay|GetRespawnActor) (Utilities|Struct|MakeS_EnemySpawn (Variables|ChildrenDefault|GetRespawnTime) (Utilities|GetClass self)))
  (Actor|DestroyActor))

(event Custom|On%20Notice%20Actor
  (params (Actor :type Actor%20Object%20Reference))
  (bind _returnvalue (AI|GetBlackboard 0))
  ;[1 1 1] SeePlayer
  (if (and (== Actor (Game|Player|GetPlayerPawn 0)) (not (Variables|Gameplay|GetSeePlayer?)))
    (bind _output_get (Variables|Gameplay|SetSeePlayer? true))
    (AI|Components|Blackboard|SetValueasBool _returnvalue (Utilities|Name|MakeLiteralName "SeePlayer?") _output_get)
    (AI|Components|Blackboard|SetValueasObject _returnvalue (Utilities|Name|MakeLiteralName "Player") (Game|Player|GetPlayerPawn 0))
    (Variables|/Script/Engine.CharacterMovementComponent|SetMaxWalkSpeed (Variables|Character|GetCharacterMovement) 5e+02)))

(event EventBeginPlay
  (bind _returnvalue (AI|GetBlackboard 0))
  ;[1 1 1] BeginPlay
  (Variables|Gameplay|SetCurrentHealth (Variables|ChildrenDefault|GetMaxHealth))
  (AI|RunBehaviorTree (AI|GetAIController self) (Variables|ChildrenDefault|GetBehaviorTree))
  (AI|Components|Blackboard|SetValueasVector _returnvalue (Utilities|Name|MakeLiteralName "OriginalLocation") (Transformation|GetActorLocation))
  (AI|Components|Blackboard|SetValueasFloat _returnvalue (Utilities|Name|MakeLiteralName "PatrolRadius") (Variables|ChildrenDefault|GetPatrolRadius))
  (AI|Components|Blackboard|SetValueasFloat _returnvalue (Utilities|Name|MakeLiteralName "AttackRange") (Variables|ChildrenDefault|GetAttackRange))
  (AI|Components|Blackboard|SetValueasFloat _returnvalue (Utilities|Name|MakeLiteralName "MovementRadius") (Variables|ChildrenDefault|GetMovementRadius))
  (CallFunction|SetupWidget))

(event Game|Damage|EventAnyDamage
  (params (Damage :type Float%20%28single-precision%29) (DamageType :type Damage%20Type%20Object%20Reference) (InstigatedBy :type Controller%20Object%20Reference) (DamageCauser :type Actor%20Object%20Reference))
  ;[1 1 1] Damage
  (if (not (Variables|Gameplay|GetIsDead?))
    (Variables|Gameplay|SetCurrentHealth (Math|Integer|Clamp(Integer) (- (Variables|Gameplay|GetCurrentHealth) (Math|Float|Round Damage)) 0 (Variables|ChildrenDefault|GetMaxHealth)))
    (CallFunction|SetupWidget)
    (if (== (Variables|Gameplay|GetCurrentHealth) 0)
      (Variables|Gameplay|SetKilledBy DamageCauser)
      (CallFunction|OnDeath)
      (else
        (CallFunction|OnNoticeActor DamageCauser)))))

(fn ConstructionScript)

(fn SetupWidget
  (bind _asenemy_widget (Utilities|Casting|CastToEnemy_Widget (UserInterface|GetUserWidgetObject (Variables|Default|GetWidget)))
    (:then
      (bind _output_get (Variables|Gameplay|SetEnemy%20Widget _asenemy_widget))
      (Rendering|Components|TextRender|SetText (Variables|/Game/QuestSystem/Blueprints/Widgets/Enemy_Widget.Enemy_Widget_C|GetNameText _output_get) (Variables|ChildrenDefault|GetName))
      (Rendering|Components|TextRender|SetText (Variables|/Game/QuestSystem/Blueprints/Widgets/Enemy_Widget.Enemy_Widget_C|GetLevelText _output_get) (Utilities|Text|ToText(Integer) (Variables|ChildrenDefault|GetLevel)))
      (CallFunction|UpdateWidgetHealth)
      (Rendering|SetVisibility (Variables|Default|GetWidget) true false))
    (:CastFailed
      (return))))

(fn UpdateWidgetHealth
  (Progress|SetPercent (Variables|/Game/QuestSystem/Blueprints/Widgets/Enemy_Widget.Enemy_Widget_C|GetHealthBar (Variables|Gameplay|GetEnemy%20Widget)) (/ (Math|Conversions|ToFloat(Integer) (Variables|Gameplay|GetCurrentHealth)) (Math|Conversions|ToFloat(Integer) (Variables|ChildrenDefault|GetMaxHealth))))
  (return))

(fn IsPlayingMontage?
  (return (Utilities|IsValid (Animation|GetCurrentMontage :!class /Script/Engine.Character))))