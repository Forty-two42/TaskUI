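; BP_GoalActor is a quest system goal marker that shows on the minimap as either an icon or a colored radius circle.
; The construction script picks which one is visible from UseRadius, then scales and tints the circle sprite from Radius and CircleColor.
; On BeginPlay it makes the player character its owner and sets Owner No See, hiding both markers from that player's own view.
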(event EventBeginPlay
  (Actor|SetOwner (Game|GetPlayerCharacter 0))
  (Class|PrimitiveComponent|SetOwnerNoSee (Variables|Default|GetMinimapIcon) true))

(event Collision|EventActorBeginOverlap
  (params (OtherActor :type Actor%20Object%20Reference)))

(event EventTick
  (params (DeltaSeconds :type Float%20%28single-precision%29)))

(fn ConstructionScript
  (bind _minimapradius (Variables|Default|GetMinimapRadius))
  (bind _radius (Variables|Default|GetRadius))
  (bind _returnvalue (/ _radius 5e+02))
  (Rendering|SetVisibility (Variables|Default|GetMinimapIcon) (not (Variables|Default|GetUseRadius?)) false)
  (Transformation|SetRelativeScale3D _minimapradius (Math|Vector|MakeVector _returnvalue 0.0 _returnvalue))
  (Rendering|SetVisibility _minimapradius (Variables|Default|GetUseRadius?) false)
  (Sprite|SetSpriteColor (Variables|Default|GetMinimapRadius) (Variables|Default|GetCircleColor)))