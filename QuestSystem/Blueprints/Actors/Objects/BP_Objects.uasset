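; BP_Objects is an interactable quest pickup actor that the player collects.
; On BeginPlay it fills its interaction widget with a pickup prompt and the name looked up from its PropsID.
; The widget shows and hides as the player enters or leaves its radius.
; On interaction it adds its class to the character's ObtainedObjects, notifies the quest manager through OnObjectFound, then destroys itself.
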(event EventBeginPlay
  (bind _asinteraction_widget (Utilities|Casting|CastToInteractionWidget (UserInterface|GetUserWidgetObject (Variables|Default|GetWidget))))
  (Rendering|Components|TextRender|SetText (Variables|/Game/QuestSystem/Blueprints/Widgets/InteractionWidget.InteractionWidget_C|GetTextBlock_Interact _asinteraction_widget) "Press [E] to Pickup")
  (bind (_found_ _prop) (CallFunction|GetPropProperty (Variables|Default|GetPropsID)))
  (if _found_
    (Rendering|Components|TextRender|SetText (Variables|/Game/QuestSystem/Blueprints/Widgets/InteractionWidget.InteractionWidget_C|GetTextBlock_Name _asinteraction_widget) (.Name (Utilities|Struct|BreakS_Props _prop)))))

(event EventOnEnterPlayerRadius
  (params (Character :type Third%20Person%20Character%20Object%20Reference))
  (Rendering|SetVisibility (Variables|Default|GetWidget) true false))

(event EventOnLeavePlayerRadius
  (params (Character :type Third%20Person%20Character%20Object%20Reference))
  (Rendering|SetVisibility (Variables|Default|GetWidget) false false))

(event EventOnInteractwith
  (params (Character :type Third%20Person%20Character%20Object%20Reference))
  (bind _self self)
  (bind _returnvalue (Utilities|GetClass _self))
  (Utilities|Array|Add (Variables|/Game/QuestSystem/Blueprints/Character/ThirdPersonCharacter.ThirdPersonCharacter_C|GetObtainedObjects Character) _returnvalue)
  (Default|OnObjectFound (Variables|/Game/QuestSystem/Blueprints/Character/ThirdPersonCharacter.ThirdPersonCharacter_C|GetQuestManagerRef Character) _returnvalue)
  (Actor|DestroyActor)
  (Utilities|Casting|CastToMyGameInstance (Game|GetGameInstance)))

(fn ConstructionScript)