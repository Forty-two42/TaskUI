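; BP_Objects_Helmet is an interactable helmet object for the quest system that goes into the inventory on interaction.
; It extends parent interaction events, creating a dynamic material on its static mesh at BeginPlay and tinting it dark blue while a character is in range, dark grey on leaving.
; Interacting looks up the prop by PropsID and, if found, adds it to the inventory through MyGameInstance.
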(event EventBeginPlay
  (bind _staticmesh (Variables|Default|GetStaticMesh))
  (|CallParentFunction)
  (Utilities|Casting|CastToInteractionWidget (UserInterface|GetUserWidgetObject (Variables|Default|GetWidget)))
  (bind _returnvalue (Rendering|Material|CreateDynamicMaterialInstance _staticmesh 0 (Rendering|Material|GetMaterial _staticmesh 0) "None" :!class /Script/Engine.PrimitiveComponent))
  (Variables|Default|SetMat_Instance _returnvalue))

(event EventOnInteractwith
  (params (Character :type Third%20Person%20Character%20Object%20Reference))
  (|CallParentFunction Character)
  (bind _asmy_game_instance (Utilities|Casting|CastToMyGameInstance (Game|GetGameInstance)))
  (bind (_found_ _prop) (CallFunction|GetPropProperty (Variables|Default|GetPropsID)))
  (if _found_
    (Default|AddInventoryItem _asmy_game_instance _prop)))

(event EventOnEnterPlayerRadius
  (params (Character :type Third%20Person%20Character%20Object%20Reference))
  (|CallParentFunction Character)
  (Rendering|Material|SetVectorParameterValue (Variables|Default|GetMat_Instance) "Color" "(R=0.000000,G=0.082353,B=0.117647,A=1.000000)" :!class /Script/Engine.MaterialInstanceDynamic))

(event EventOnLeavePlayerRadius
  (params (Character :type Third%20Person%20Character%20Object%20Reference))
  (|CallParentFunction Character)
  (Rendering|Material|SetVectorParameterValue (Variables|Default|GetMat_Instance) "Color" "(R=0.027451,G=0.027451,B=0.027451,A=1.000000)" :!class /Script/Engine.MaterialInstanceDynamic))

(fn ConstructionScript
  (|CallParentFunction))