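; Blueprint function library of helpers for the task (quest) system, covering UI display data and DataTable lookups.
; One function maps a task's main type (mainline, branchline, repeated, daily, challenge) to an image, color and Chinese label.
; Others convert a numeric ID to a row name and fetch task info, kill-enemy targets or get-prop targets from separate DataTables.
; The talk-target getter is an empty stub.
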(fn GetTaskUIDatabyMainType
  (params (MainType :type E_TaskMainType%20Enum :default "NewEnumerator0"))
  (return (Utilities|Select :Index MainType :NewEnumerator0 "/Game/Mannequin/Character/Materials/MaterialLayers/T_ML_Rubber_Blue_01_N.T_ML_Rubber_Blue_01_N" :NewEnumerator1 "/Game/Mannequin/Character/Materials/MaterialLayers/T_ML_Aluminum01_N.T_ML_Aluminum01_N" :NewEnumerator2 "/Game/Mannequin/Character/Textures/T_UE4Logo_N.T_UE4Logo_N" :NewEnumerator3 "/Game/Mannequin/Character/Textures/T_UE4Logo_Mask.T_UE4Logo_Mask" :NewEnumerator4 "/Game/Mannequin/Character/Materials/MaterialLayers/T_ML_Aluminum01.T_ML_Aluminum01") (Math|Conversions|ToLinearColor(Color) (Utilities|Select :Index MainType :NewEnumerator0 "" :NewEnumerator1 "" :NewEnumerator2 "" :NewEnumerator3 "" :NewEnumerator4 "")) (Utilities|Select :Index MainType :NewEnumerator0 "主线" :NewEnumerator1 "支线" :NewEnumerator2 "重复" :NewEnumerator3 "日常" :NewEnumerator4 "挑战")))

(fn GetTaskDatatableInfo
  (params (ID :type Integer))
  (bind _returnvalue (Utilities|GetDataTableRow "/Game/UI/Task/DT_Task.DT_Task" (Utilities|String|StringToName (Utilities|String|ToString(Integer) ID)))
    (:then
      (return _returnvalue))))

(fn GetTaskTargetKillEnemies
  (params (TaskID :type Integer))
  (bind _returnvalue (Utilities|GetDataTableRow "/Game/UI/Task/DT_TaskTarget_Enemies.DT_TaskTarget_Enemies" (Utilities|String|StringToName (Utilities|String|ToString(Integer) TaskID)))
    (:then
      (return _returnvalue))))

(fn GetTaskTargetGetprops
  (params (TaskID :type Integer))
  (bind _returnvalue (Utilities|GetDataTableRow "/Game/UI/Task/DT_TaskTarget_GetProps.DT_TaskTarget_GetProps" (Utilities|String|StringToName (Utilities|String|ToString(Integer) TaskID)))
    (:then
      (return _returnvalue))))

(fn GetTaskTargetTalk)