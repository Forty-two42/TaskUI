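; BP_Player is the player Blueprint that handles talking to NPCs and opening the task message.
; Box overlaps with BP_NPC toggle the player action state, track the facing NPC and show or hide a dialog tip through the controller.
; Pressing Talk while nearly stationary looks up that NPC in DT_NPC by enum name and sends its first dialog entry, thumbnail, name and task ID to the controller.
; CallTask asks the controller to show tasks.
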(event OnComponentBeginOverlap(Box)
  (params (OverlappedComponent :type Primitive%20Component%20Object%20Reference) (OtherActor :type Actor%20Object%20Reference) (OtherComp :type Primitive%20Component%20Object%20Reference) (OtherBodyIndex :type Integer) (bFromSweep :type Boolean) (SweepResult :type Hit%20Result%20Structure%20%28by%20ref%29))
  (bind _asbp_npc (Utilities|Casting|CastToBP_NPC OtherActor))
  (if (Utilities|Enum|Equal(Enum) (Variables|Default|GetPlayerAction) "NewEnumerator0")
    (Variables|Default|SetPlayerAction "NewEnumerator1")
    (Variables|Default|SetCurrentFaceNPC _asbp_npc)
    (Class|InterfacePlayerController|ShowDialogTIp(Message) (Pawn|GetController) true)))

(event OnComponentEndOverlap(Box)
  (params (OverlappedComponent :type Primitive%20Component%20Object%20Reference) (OtherActor :type Actor%20Object%20Reference) (OtherComp :type Primitive%20Component%20Object%20Reference) (OtherBodyIndex :type Integer))
  (bind _asbp_npc (Utilities|Casting|CastToBP_NPC OtherActor))
  (if (and (== _asbp_npc (Variables|Default|GetCurrentFaceNPC)) (Utilities|Enum|Equal(Enum) (Variables|Default|GetPlayerAction) "NewEnumerator1"))
    (Variables|Default|SetPlayerAction "NewEnumerator0")
    (Variables|Default|SetCurrentFaceNPC _asbp_npc)
    (Class|InterfacePlayerController|ShowDialogTIp(Message) (Pawn|GetController) false)))

(event EventBeginPlay)

(event Collision|EventActorBeginOverlap
  (params (OtherActor :type Actor%20Object%20Reference)))

(event EventTick
  (params (DeltaSeconds :type Float%20%28single-precision%29)))

(event Input|ActionEvents|InputActionTalk
  (params (Key :type Key%20Structure :default "None"))
  (:Pressed
    (if (and (Utilities|Enum|Equal(Enum) (Variables|Default|GetPlayerAction) "NewEnumerator1") (< (Math|Vector|VectorLength (Transformation|GetVelocity)) 0.1))
      (Utilities|IsValid (Variables|Default|GetCurrentFaceNPC)
        (:Is%20Valid
          (bind (_outarray _taskid _thumbnail _npc_name) (CallFunction|GetDialogArray))
          (Class|InterfacePlayerController|ShowDialog(Message) (Pawn|GetController) _thumbnail _npc_name _outarray _taskid))))))

(event Input|ActionEvents|InputActionCallTask
  (params (Key :type Key%20Structure :default "None"))
  (:Pressed
    (Class|InterfacePlayerController|ShowTask(Message) (Pawn|GetController))))

(fn ConstructionScript
  (|CallParentFunction))

(fn GetDialogArray
  (bind _currentfacenpc (Variables|Default|GetCurrentFaceNPC))
  (Utilities|IsValid _currentfacenpc
    (:Is%20Valid
      (bind _returnvalue (Utilities|GetDataTableRow "/Game/Blueprints/NPC/DT_NPC.DT_NPC" (Utilities|String|StringToName (Utilities|String|EnumtoString (Variables|/Game/Blueprints/NPC/BP_NPC.BP_NPC_C|GetName _currentfacenpc))))
        (:then
          (for _array_element (.AllDialog (Utilities|Struct|BreakS_NPC_Info _returnvalue))
            _)
          (return (.Dialog (Utilities|Struct|BreakS_Dialog_Task (Utilities|Array|Get(acopy) (.AllDialog (Utilities|Struct|BreakS_NPC_Info _returnvalue))))) (.Task_ID (Utilities|Struct|BreakS_Dialog_Task (Utilities|Array|Get(acopy) (.AllDialog (Utilities|Struct|BreakS_NPC_Info _returnvalue))))) (.Thumbnail (Utilities|Struct|BreakS_NPC_Info _returnvalue)) (Utilities|Text|ToText(String) (Utilities|String|EnumtoString (.Name (Utilities|Struct|BreakS_NPC_Info _returnvalue))))))))))