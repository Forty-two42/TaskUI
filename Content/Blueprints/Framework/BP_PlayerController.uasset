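; BP_PlayerController is the player controller that creates the main HUD widget and acts as the bridge to its dialog and quest (task) UI.
; BeginPlay adds W_Main to the viewport, and interface events forward calls to its child widgets to toggle the dialog tip, start NPC dialog, update task details or toggle the task list.
; Opening dialog or the task list switches to Game-and-UI input with a cursor; dialog also blocks movement.
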(event EventBeginPlay
  (bind _returnvalue (UserInterface|CreateWidget "/Game/UI/W_Main.W_Main_C" self))
  (bind _output_get (Variables|Default|SetMainUI _returnvalue))
  (UserInterface|Viewport|AddtoViewport _output_get 0))

(event EventTick
  (params (DeltaSeconds :type Float%20%28single-precision%29)))

(event EventShowDialog
  (params (Thunbnail :type Texture%202D%20Object%20Reference) (Name :type Text) (DialogArray :type Array%20of%20S%20Dialog%20Structures) (TaskID :type Integer))
  (bind _mainui (Variables|Default|GetMainUI)
    (:then
      (Default|InitDialog (Variables|/Game/UI/W_Main.W_Main_C|GetW_Dialog _mainui) Thunbnail Name DialogArray TaskID)
      (Input|SetInputModeGameandUI self 0 "DoNotLock" true)
      (Variables|Default|SetbShowMouseCursor true)
      (Input|SetIgnoreMoveInput true))
    (:else)))

(event EventShowDialogTIp
  (params (Open :type Boolean))
  (bind _mainui (Variables|Default|GetMainUI)
    (:then
      (if Open
        (Widget|SetVisibility (Variables|/Game/UI/Dialog/W_Dialog.W_Dialog_C|GetTextBlock_DialogTip (Variables|/Game/UI/W_Main.W_Main_C|GetW_Dialog _mainui)) "SelfHitTestInvisible")
        (else
          (Widget|SetVisibility (Variables|/Game/UI/Dialog/W_Dialog.W_Dialog_C|GetTextBlock_DialogTip (Variables|/Game/UI/W_Main.W_Main_C|GetW_Dialog _mainui)) "Collapsed"))))
    (:else)))

(event EventShowTask
  (bind _mainui (Variables|Default|GetMainUI)
    (:then
      (if (Widget|IsVisible (Variables|/Game/UI/W_Main.W_Main_C|GetW_AllTask _mainui))
        (Widget|SetVisibility (Variables|/Game/UI/W_Main.W_Main_C|GetW_AllTask _mainui) "Collapsed")
        (else
          (Widget|SetVisibility (Variables|/Game/UI/W_Main.W_Main_C|GetW_AllTask _mainui) "SelfHitTestInvisible")
          (Input|SetInputModeGameandUI self 0 "DoNotLock" true)
          (Variables|Default|SetbShowMouseCursor true))))
    (:else)))

(event EventShowTaskDetail
  (params (TaskInfo :type S%20Task%20Structure))
  (bind (_id _name _description _requiredlevel _maintype) (Utilities|Struct|BreakS_Task TaskInfo))
  (bind _mainui (Variables|Default|GetMainUI)
    (:then
      (if (!= (.ID (Utilities|Struct|BreakS_Task TaskInfo)) (.ID (Utilities|Struct|BreakS_Task (Variables|/Game/UI/Task/W_TaskDetail.W_TaskDetail_C|GetTaskInfo (Variables|/Game/UI/Task/W_AllTask.W_AllTask_C|GetW_TaskDetail (Variables|/Game/UI/W_Main.W_Main_C|GetW_AllTask _mainui))))))
        (Default|TaskClick (Variables|/Game/UI/W_Main.W_Main_C|GetW_AllTask _mainui) _maintype _id)
        (Default|SetTaskDetail (Variables|/Game/UI/Task/W_AllTask.W_AllTask_C|GetW_TaskDetail (Variables|/Game/UI/W_Main.W_Main_C|GetW_AllTask _mainui)) TaskInfo)))
    (:else)))

(fn ConstructionScript)